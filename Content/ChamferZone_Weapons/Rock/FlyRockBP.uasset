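; Flying rock projectile Blueprint that bounces off surfaces with impact effects.
; A timeline started on BeginPlay drives the projectile movement's max speed over time.
; The first two bounces sphere-trace the hit point to branch on physical material, then spawn an emitter, randomly tilted around the impact normal, and a sound.
; When the projectile stops, it destroys its FlyBullet component after a short delay.
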(event `self.ProjectileMovement.OnProjectileStop`
  (params (ImpactResult :type "HitResult Structure (by ref)"))
  (`KismetSystemLibrary.Delay` 2.0)
  (`ActorComponent.K2_DestroyComponent` (`self.FlyBullet`)))

(event `self.ProjectileMovement.OnProjectileBounce`
  (params (ImpactResult :type "HitResult Structure (by ref)") (ImpactVelocity :type "Vector Structure (by ref)"))
  (bind (_bblockinghit _binitialoverlap _time _distance _location _impactpoint _normal _impactnormal) (`GameplayStatics.BreakHitResult` ImpactResult))
  (if (<= (`self.BounchTime`) 1)
    (set `self.BounchTime` (+ (`self.BounchTime`) 1))
    (bind _outhit (`KismetSystemLibrary.SphereTraceSingle` _location _location 10.0 "TraceTypeQuery1"))
    (bind (_bblockinghit_2 _binitialoverlap_2 _time_2 _distance_2 _location_2 _impactpoint_2 _normal_2 _impactnormal_2 _physmat) (`GameplayStatics.BreakHitResult` _outhit))
    (if (== _physmat null)
      (set `self.Paricitle` null)
      (set `self.Sound` null)
      (elif (== _physmat null)
        (set `self.Paricitle` null)
        (set `self.Sound` null)
        (elif (== _physmat null)
          (set `self.Paricitle` null)
          (set `self.Sound` null))))
    (`GameplayStatics.SpawnEmitterAtLocation` (`self.Paricitle`) _location (`KismetMathLibrary.MakeRotFromZ` (* (`KismetMathLibrary.RandomUnitVectorInConeInRadians` (`KismetMathLibrary.GetDirectionUnitVector` _impactnormal) 0.25) -1.0)))
    (`GameplayStatics.SpawnSoundAtLocation` (`self.Sound`) _location (struct) 1.0 1.0 0.0 null null)))

(event `self.ReceiveBeginPlay`
  (bind (_direction _value) (`Timeline|时间轴_0`)
    (:`Update`
      (set `ProjectileMovementComponent.MaxSpeed` _value (`self.ProjectileMovement`)))))

(fn `UserConstructionScript`)