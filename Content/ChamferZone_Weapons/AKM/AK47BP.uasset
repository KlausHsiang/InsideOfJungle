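; AK-47 weapon actor for the ALS player character that picks one of four random skin materials on BeginPlay.
; Fire traces from the third-person camera, then launches a bullet actor from the muzzle toward the hit with random spread, or along camera rotation without spread on a miss.
; Each shot plays effects, ejects a shell and raises a clamped bloom value, which scales spread with AimValue and decays on Tick after firing stops.
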(event `self.ReceiveBeginPlay`
  (bind _returnvalue (`KismetMathLibrary.RandomBool`))
  (if (`KismetMathLibrary.RandomBool`)
    (if _returnvalue
      (set `self.Mat` "/Game/ChamferZone_Weapons/AKM/WPNM_AKM_Inst.WPNM_AKM_Inst")
      (else
        (set `self.Mat` "/Game/ChamferZone_Weapons/AKM/WPNM_AKM_Inst1.WPNM_AKM_Inst1")))
    (elif _returnvalue
      (set `self.Mat` "/Game/ChamferZone_Weapons/AKM/WPNM_AKM_Inst2.WPNM_AKM_Inst2")
      (else
        (set `self.Mat` "/Game/ChamferZone_Weapons/AKM/WPNM_AKM_Inst3.WPNM_AKM_Inst3"))))
  (`PrimitiveComponent.SetMaterial` (`self.SkeletalMesh`) 0 (`self.Mat`)))

(event `Fire`
  (bind _arrow (`self.Arrow`))
  (bind _skeletalmesh (`self.SkeletalMesh`))
  (bind _returnvalue (`SceneComponent.K2_GetComponentLocation` (`self.Arrow`)))
  (bind _asals_base_character (cast `/Game/MainFemaleCharacter/Blueprints/ALS_BaseCharacter` (`GameplayStatics.GetPlayerCharacter` 0)))
  (set `self.IsFire` true)
  (bind _tp_camera (`/Game/MainFemaleCharacter/Blueprints/ALS_BaseCharacter.TP_Camera` _asals_base_character))
  (bind _returnvalue_2 (`SceneComponent.K2_GetComponentLocation` _tp_camera))
  (bind _returnvalue_3 (`SceneComponent.K2_GetComponentRotation` _tp_camera))
  (bind (_outhit _returnvalue_4) (`KismetSystemLibrary.LineTraceSingle` _returnvalue_2 (+ _returnvalue_2 (* (`KismetMathLibrary.GetForwardVector` _returnvalue_3) 8000.0)) "TraceTypeQuery1"))
  (if _returnvalue_4
    (bind _returnvalue_5 (* (`/Game/MainFemaleCharacter/Blueprints/ALS_BaseCharacter.AimValue` _asals_base_character) (`self.ShootValue`)))
    (bind _returnvalue_6 (* _returnvalue_5 -1.0))
    (set `self.BulletTra` (`KismetMathLibrary.MakeTransform` _returnvalue (`KismetMathLibrary.MakeRotator` (+ (.roll (`KismetMathLibrary.FindLookAtRotation` _returnvalue (`.Location` (`GameplayStatics.BreakHitResult` _outhit)))) (`KismetMathLibrary.RandomFloatInRange` _returnvalue_6 _returnvalue_5)) (+ (.pitch (`KismetMathLibrary.FindLookAtRotation` _returnvalue (`.Location` (`GameplayStatics.BreakHitResult` _outhit)))) (`KismetMathLibrary.RandomFloatInRange` _returnvalue_6 _returnvalue_5)) (+ (.yaw (`KismetMathLibrary.FindLookAtRotation` _returnvalue (`.Location` (`GameplayStatics.BreakHitResult` _outhit)))) (`KismetMathLibrary.RandomFloatInRange` _returnvalue_6 _returnvalue_5)))))
    (else
      (set `self.BulletTra` (`KismetMathLibrary.MakeTransform` _returnvalue _returnvalue_3))))
  (`AnimInstance.Montage_Play` (`SkeletalMeshComponent.GetAnimInstance` (`self.SkeletalMesh`)) "/Game/ChamferZone_Weapons/AKM/AK47Fire_Montage.AK47Fire_Montage" 1.0 "MontageLength" 0.0 true)
  (`GameplayStatics.SpawnSoundAttached` "/Game/ChamferZone_Weapons/AKM/AK47Sound.AK47Sound" _skeletalmesh "None" (0.0 0.0 0.0) (struct) "KeepRelativeOffset" false 1.0 1.0 0.0 null null)
  (`GameplayStatics.SpawnSoundAttached` "/Game/ChamferZone_Weapons/AKM/AK47Sound_2.AK47Sound_2" _skeletalmesh "None" (0.0 0.0 0.0) (struct) "KeepRelativeOffset" false 1.0 1.0 0.0 null null)
  (`GameplayStatics.SpawnEmitterAttached` null _arrow)
  (`GameplayStatics.SpawnEmitterAttached` null _arrow)
  (`|SpawnActorFromClass` "/Game/ChamferZone_Weapons/AKM/FlyBulletBP.FlyBulletBP_C" (`self.BulletTra`) "Undefined" "OverrideRootScale" null null)
  (`|SpawnActorFromClass` "/Game/ChamferZone_Weapons/AKM/7-62BulletBP.7-62BulletBP_C" (`SceneComponent.GetSocketTransform` (`self.ArrowShell`) "None" "RTS_World") "Undefined" "OverrideRootScale" null null)
  (set `self.ShootValue` (`KismetMathLibrary.FClamp` (+ (`self.ShootValue`) 0.3) 0.0 5.0))
  (`KismetSystemLibrary.RetriggerableDelay` 0.6)
  (set `self.IsFire` false))

(event `self.ReceiveTick`
  (params (DeltaSeconds :type "Float (single-precision)"))
  (bind _shootvalue (`self.ShootValue`))
  (if (not (`self.IsFire`))
    (`KismetSystemLibrary.Delay` 0.01)
    (if (>= _shootvalue 0.0)
      (set `self.ShootValue` (- _shootvalue 0.1)))))

(fn `UserConstructionScript`)